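; BP_Player2 is a player character Blueprint that adds a blink-dash evade on the Evade input, usable only while movement input is held.
; Pressing Evade plays an effort voice cue and runs the blinkDashFX macro with the movement component, capsule, camera and a wind Niagara effect.
; When the dash outputs, it stops the current montage and ends the equipped weapon's attack, while Tick feeds the same dash macro each frame.
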(event `InputAction|Evade`
  (params (Key :type "Key Structure"))
  (:`Pressed`
    (if (not (and (== (`self.GetInputAxisValue`) 0.0) (== (`self.GetInputAxisValue`) 0.0)))
      (`GameplayStatics.PlaySound2D` "/Game/HumanVocalizations/HumanFemaleC/Cues/voice_female_c_effort_jump_01_Cue.voice_female_c_effort_jump_01_Cue" 0.5 1.0 0.0 null null false)
      (`/Game/BlinkAndDashVFX/BluePrints/DashFX_MacrosLibrary.BlinkDashFX` (`self.CharacterMovement`) 500.0 "/Game/BlinkAndDashVFX/VFX_Niagara/NS_Dash_Wind.NS_Dash_Wind" null self (`self.CapsuleComponent`) 0.4 0.0 (`self.MeshCamera`) :!label _label
        (:`Out`
          (`self.StopAnimMontage` null)
          (`CEquipItem.EndAttack` (`CItemData.GetEquipItem` (`CWeaponComponent.GetCurrentWeapon` (`self.WeaponComponent`)))))))))

(event `self.ReceiveTick`
  (params (DeltaSeconds :type "Float (single-precision)"))
  (goto _label :!via `EventTick`))

(fn `UserConstructionScript`)